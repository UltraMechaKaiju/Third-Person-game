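; Grind rail actor that builds its visible, collidable rail along the GrindRail spline in the Construction Script.
; Each segment gets a custom spline mesh component using SplineTestMesh on a Z forward axis, fitted to local positions and tangents with world-space roll.
; Segments generate overlaps on a custom trace channel object type, presumably for grind detection.
; Closed-loop splines get an extra closing segment; there is no runtime logic.
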(event EventBeginPlay)

(event Collision|EventActorBeginOverlap
  (params (OtherActor :type Actor%20Object%20Reference)))

(event EventTick
  (params (DeltaSeconds :type Float%20%28single-precision%29)))

(fn ConstructionScript
  (bind _grindrail (Variables|Default|GetGrindRail))
  (bind _returnvalue (Spline|GetNumberOfSplinePoints _grindrail))
  (if (Class|SplineComponent|IsClosedLoop _grindrail)
    (for _index (range 0 (- _returnvalue 1))
      (bind _returnvalue_2 (AddComponent|AddCustomSplineMeshComponent false))
      (Components|StaticMesh|SetStaticMesh _returnvalue_2 "/Game/Mesh/SplineTestMesh.SplineTestMesh")
      (SplineMesh|SetStartandEnd _returnvalue_2 (Spline|GetLocationatSplinePoint _grindrail _index "Local") (Spline|GetTangentatSplinePoint _grindrail _index "Local") (Spline|GetLocationatSplinePoint _grindrail (+ _index 1) "Local") (Spline|GetTangentatSplinePoint _grindrail (+ _index 1) "Local") true :!class /Script/Engine.SplineMeshComponent)
      (SplineMesh|SetEndRollDegrees _returnvalue_2 (Spline|GetRollatSplinePoint _grindrail (+ _index 1) "World") true)
      (SplineMesh|SetStartRollDegrees _returnvalue_2 (Spline|GetRollatSplinePoint _grindrail _index "World") true)
      (Variables|/Script/Engine.PrimitiveComponent|SetbGenerateOverlapEvents _returnvalue_2 true)
      (Collision|SetCollisionEnabled _returnvalue_2 "QueryAndPhysics")
      (SplineMesh|SetForwardAxis _returnvalue_2 "Z" true)
      (Collision|SetCollisionObjectType _returnvalue_2 "ECC_GameTraceChannel1"))
    (else
      (for _index_2 (range 0 (- _returnvalue 2))
        (bind _returnvalue_3 (AddComponent|AddCustomSplineMeshComponent false))
        (Components|StaticMesh|SetStaticMesh _returnvalue_3 "/Game/Mesh/SplineTestMesh.SplineTestMesh")
        (SplineMesh|SetStartandEnd _returnvalue_3 (Spline|GetLocationatSplinePoint _grindrail _index_2 "Local") (Spline|GetTangentatSplinePoint _grindrail _index_2 "Local") (Spline|GetLocationatSplinePoint _grindrail (+ _index_2 1) "Local") (Spline|GetTangentatSplinePoint _grindrail (+ _index_2 1) "Local") true :!class /Script/Engine.SplineMeshComponent)
        (SplineMesh|SetStartRollDegrees _returnvalue_3 (Spline|GetRollatSplinePoint _grindrail _index_2 "World") true)
        (SplineMesh|SetEndRollDegrees _returnvalue_3 (Spline|GetRollatSplinePoint _grindrail (+ _index_2 1) "World") true)
        (Variables|/Script/Engine.PrimitiveComponent|SetbGenerateOverlapEvents _returnvalue_3 true)
        (Collision|SetCollisionEnabled _returnvalue_3 "QueryAndPhysics")
        (SplineMesh|SetForwardAxis _returnvalue_3 "Z" true)
        (Collision|SetCollisionObjectType _returnvalue_3 "ECC_GameTraceChannel1")))))