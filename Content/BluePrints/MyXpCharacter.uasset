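; Player character Blueprint that uses a movement component with skate gravity and sprint functions, holding test and debug logic.
; The only live behavior zeroes the movement component's velocity when the right mouse button is pressed.
; Unconnected leftover nodes would set skate gravity and walking mode, toggle sprint, and print squared speed and movement mode.
; Tick and the construction script are empty.
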(event EventTick
  (params (DeltaSeconds :type Float%20%28single-precision%29)))

(event Input|KeyboardEvents|LeftShift
  (params (Key :type Key%20Structure :default "None")))

(event Input|KeyboardEvents|RightShift
  (params (Key :type Key%20Structure :default "None")))

(event Input|MouseEvents|RightMouseButton
  (params (Key :type Key%20Structure :default "None"))
  (:Pressed
    (Variables|/Script/Engine.MovementComponent|SetVelocity (Variables|Default|GetMovementComponent) "0, 0, 0")))

(fn ConstructionScript)