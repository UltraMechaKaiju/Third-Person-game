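; MyStatue is a Blueprint actor for a statue that moves in response to the proximity of MyXpCharacter.
; Entering SmallerColl starts the Move component forward, and leaving BiggerColl reverses it, with the two volumes giving separate trigger and release ranges.
; The Shouldnotmove flag lets the non-top endpoint event stop and reset the movement after the character leaves.
; A separate Collect event plays an explosion sound.
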(event OnComponentBeginOverlap(SmallerColl)
  (params (OverlappedComponent :type Primitive%20Component%20Object%20Reference) (OtherActor :type Actor%20Object%20Reference) (OtherComp :type Primitive%20Component%20Object%20Reference) (OtherBodyIndex :type Integer) (bFromSweep :type Boolean) (SweepResult :type Hit%20Result%20Structure%20%28by%20ref%29))
  (bind _move (Variables|Default|GetMove))
  (Utilities|Casting|CastToMyXpCharacter OtherActor)
  (Class|MoveComponent|EnableMovement _move true)
  (Class|MoveComponent|SetDirection _move 1)
  (Variables|Default|Setshouldnotmove false))

(event OnEndPointReached(Move)
  (params (IsTopEndpoint :type Boolean))
  (bind _move (Variables|Default|GetMove))
  (if (and (not IsTopEndpoint) (Variables|Default|Getshouldnotmove))
    (Class|MoveComponent|EnableMovement _move false)
    (Class|MoveComponent|MoveReset _move)))

(event OnComponentEndOverlap(BiggerColl)
  (params (OverlappedComponent :type Primitive%20Component%20Object%20Reference) (OtherActor :type Actor%20Object%20Reference) (OtherComp :type Primitive%20Component%20Object%20Reference) (OtherBodyIndex :type Integer))
  (Utilities|Casting|CastToMyXpCharacter OtherActor)
  (Class|MoveComponent|SetDirection (Variables|Default|GetMove) -1)
  (Variables|Default|Setshouldnotmove true))

(event EventCollect
  (params (SourceObject :type Object%20Object%20Reference) (Count :type Float%20%28single-precision%29))
  (bind _explosion (Variables|Default|GetExplosion))
  (Audio|Components|Audio|SetSound _explosion "/Game/StarterContent/Audio/Explosion01.Explosion01")
  (Audio|Components|Audio|Play _explosion 0.0))

(event Collision|EventActorBeginOverlap
  (params (OtherActor :type Actor%20Object%20Reference)))

(event EventTick
  (params (DeltaSeconds :type Float%20%28single-precision%29)))

(fn ConstructionScript)

(fn NewFunction)